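; BP_NPC is an NPC that patrols a looping path of waypoints.
; On BeginPlay it converts the Path points from actor-relative to world space into TransformedPath, prints a debug position and starts patrolling.
; Patrol uses AIMoveTo, waits for Duration on success, then NextWayPoint advances the index, wrapping to the first point, and calls Patrol again.
; A failed move has no handler, so it ends the loop.
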(event `self.ReceiveBeginPlay`
  (for _array_element (`self.Path`)
    (bind _returnvalue (`KismetMathLibrary.TransformLocation` (`self.GetTransform`) _array_element))
    (`KismetArrayLibrary.Array_Add` (`self.Transformed Path`) _returnvalue))
  (set `self.Current Way Point` (`|GetArrayItem` (`self.Transformed Path`)))
  (`KismetSystemLibrary.PrintString` (`KismetStringLibrary.Conv_VectorToString` _returnvalue))
  (`self.Patrol`))

(event `Patrol`
  (`|AIMoveTo` self (`self.Current Way Point`) null
    (:`OnSuccess`
      (`KismetSystemLibrary.Delay` (`self.Duration`))
      (`self.Next Way Point`))))

(event `Next Way Point`
  (if (< (`self.Current Path Index`) (- (`KismetArrayLibrary.Array_Length` (`self.Transformed Path`)) 1))
    (bind _result (`/Engine/EditorBlueprintResources/StandardMacros.IncrementInt` (`self.Current Path Index`))
      (:`  `
        (set `self.Current Way Point` (`|GetArrayItem` (`self.Transformed Path`) _result))))
    (else
      (set `self.Current Path Index` 0)
      (set `self.Current Way Point` (`|GetArrayItem` (`self.Transformed Path`)))))
  (`self.Patrol`))

(fn `UserConstructionScript`)